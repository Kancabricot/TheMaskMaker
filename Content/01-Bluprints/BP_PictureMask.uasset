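; BP_PictureMask takes scene captures from up to three preset poses, storing them in a series of render targets.
; ScreenMask starts at the first pose; each TakePicture captures there, increments the index, then switches to that index's render target and pose for the next shot.
; The index has no bounds check or reset, a debug string prints per capture, and the pose-array setup is unconnected.
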(event Custom|TakePicture
  (Rendering|SceneCapture|CaptureScene (Variables|Default|GetScreenMask) :!class /Script/Engine.SceneCaptureComponent2D)
  (bind _output_get (Variables|Default|SetPictureIndex (+ (Variables|Default|GetPictureIndex) 1)))
  (Development|PrintString (Utilities|String|Append (Utilities|String|ToString(Integer) _output_get) " 
KIHGFLIYKLHJKM") true true "(R=1.000000,G=0.000000,B=0.266438,A=1.000000)" 5.0)
  (Variables|/Script/Engine.SceneCaptureComponent2D|SetTextureTarget (Variables|Default|GetScreenMask) (Utilities|Array|Get(acopy) (Variables|Default|GetTextureTargetArray) _output_get))
  (Transformation|SetWorldLocationAndRotation (Variables|Default|GetScreenMask) (Transformation|GetWorldLocation (Utilities|Select :Index (Variables|Default|GetPictureIndex) :Option%200 (Variables|Default|GetScenePose1) :Option%201 (Variables|Default|GetScenePose2) :Option%202 (Variables|Default|GetScenePose3))) (Transformation|GetWorldRotation (Utilities|Select :Index (Variables|Default|GetPictureIndex) :Option%200 (Variables|Default|GetScenePose1) :Option%201 (Variables|Default|GetScenePose2) :Option%202 (Variables|Default|GetScenePose3))) false false))

(event EventBeginPlay
  (bind _scenepose1 (Variables|Default|GetScenePose1))
  (Transformation|SetWorldLocationAndRotation (Variables|Default|GetScreenMask) (Transformation|GetWorldLocation _scenepose1) (Transformation|GetWorldRotation _scenepose1) false false))

(fn ConstructionScript)
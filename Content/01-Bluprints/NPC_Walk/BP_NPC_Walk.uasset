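; NPC walker Blueprint that follows the points of a referenced spline and destroys itself once its index exceeds the point count.
; On BeginPlay it registers itself with its AIC_NPC_Walk controller, caches the spline and calls NextPoint.
; NextPoint, gated by a moving flag it sets but never clears here, increments the index and passes that point's world location to the controller's MoveToNextPoint.
; A spline-based rotation step is left disconnected.
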(event Custom|Next%20Point
  (if (not (Variables|Default|Getb_isMoving))
    (bind _output_get (Variables|Default|SetPoinr%20Index (+ (Variables|Default|GetPoinr%20Index) 1)))
    (Development|PrintString (Utilities|String|ToString(Integer) _output_get))
    (if (<= _output_get (Spline|GetNumberOfSplinePoints (Variables|Default|GetSpline)))
      (Variables|Default|Setb_isMoving true)
      (Default|MovetoNextPoint (Variables|Default|GetAs%20AIC%20NPC%20Walk) (Spline|GetLocationatSplinePoint (Variables|Default|GetSpline) (Variables|Default|GetPoinr%20Index) "World"))
      (else
        (Actor|DestroyActor)))))

(event EventBeginPlay
  (bind _asaic_npc_walk (Utilities|Casting|CastToAIC_NPC_Walk (AI|GetAIController self))
    (:then
      (Variables|/Game/01-Bluprints/NPC_Walk/AIC_NPC_Walk.AIC_NPC_Walk_C|SetControlled%20NPC _asaic_npc_walk self)
      (Variables|Default|SetSpline (Variables|/Game/01-Bluprints/NPC_Walk/BP_NPCWalk_Spline.BP_NPCWalk_Spline_C|GetSpline (Variables|Default|GetSpline%20Ref)))
      (Variables|Default|SetAs%20AIC%20NPC%20Walk _asaic_npc_walk)
      (CallFunction|NextPoint))
    (:CastFailed
      (Development|PrintString "Cast Failed"))))

(fn ConstructionScript)
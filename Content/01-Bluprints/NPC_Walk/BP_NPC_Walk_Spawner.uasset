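; BP_NPC_Walk_Spawner periodically spawns BP_NPC_Walk actors at its own transform, handing each its Spline reference.
; BeginPlay starts a looping timer at SpawnInterval that calls SpawnNPC, which spawns only while the spline is valid.
; Each spawn randomizes SpawnInterval, but the running timer is never reset, so its period stays fixed.
; StopSpawn clears and invalidates the timer.
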(event Custom|Spawn%20NPC
  (Variables|Default|GetSpline
    (:then
      (Game|SpawnActorfromClass "/Game/01-Bluprints/NPC_Walk/BP_NPC_Walk.BP_NPC_Walk_C" (Transformation|GetActorTransform) "Undefined" "MultiplyWithRoot" 0 (Variables|Default|GetSpline) 0)
      (Variables|Default|SetSpawn%20Interval (Math|Random|RandomFloatinRange 3.0 8.0)))
    (:else)))

(event Custom|Stop%20Spawn
  (bind _spawn_timer_handle (Variables|Default|GetSpawn%20Timer%20Handle))
  (if (Utilities|Time|IsValidTimerHandle _spawn_timer_handle)
    (Utilities|Time|ClearandInvalidateTimerbyHandle _spawn_timer_handle)))

(event EventBeginPlay
  (bind _returnvalue (Utilities|Time|SetTimerbyEvent (delegate Custom|Spawn%20NPC) (Variables|Default|GetSpawn%20Interval) true false -1.0))
  (Variables|Default|SetSpawn%20Timer%20Handle _returnvalue))

(fn ConstructionScript)
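; Path route Blueprint that holds an ordered PathPos array for defined-path NPC movement.
; On BeginPlay it resets its index and, if its own AI controller casts to AIc_npcDefinedPath, registers itself as that controller's MyPathPoint.
; SetPos takes the last index and returns the next path entry with its index, without bounds checking or wraparound.
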(event EventBeginPlay
  (Variables|Default|SetIndex 0)
  (bind _asaic_npc_defined_path (Utilities|Casting|CastToAIc_npcDefinedPath (AI|GetAIController self)))
  (Variables|/Game/01-Bluprints/Entity/NpcDefinedPath/AIc_npcDefinedPath.AIc_npcDefinedPath_C|SetMyPathPoint _asaic_npc_defined_path self))

(fn ConstructionScript)

(fn SetPos
  (params (My%20NpcDefinedPath :type Bp%20Npc%20Defined%20Path%20Object%20Reference) (LastPos :type Integer))
  (bind _output_get (Variables|Default|SetIndex (+ LastPos 1)))
  (return (Utilities|Array|Get(acopy) (Variables|Default|GetPathPos) _output_get) _output_get))
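; Player Blueprint with walk, look, overlap-based interaction and a toggleable paint mode for a mask plane.
; Paint mode shows the WG_Paint widget and cursor, moves the camera to the plane's arrow and disables look.
; While click is held, mouse traces drive an interpolated Cube as the brush.
; Leaving paint mode restores the camera, resets the Cube and asks BP_RVT_Volume to calculate color percentage.
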(event OnComponentBeginOverlap(CapsuleInteract)
  (params (OverlappedComponent :type Primitive%20Component%20Object%20Reference) (OtherActor :type Actor%20Object%20Reference) (OtherComp :type Primitive%20Component%20Object%20Reference) (OtherBodyIndex :type Integer) (bFromSweep :type Boolean) (SweepResult :type Hit%20Result%20Structure%20%28by%20ref%29))
  ;[1 1 1] Interact
  (bind _asbp_interact (Utilities|Casting|CastToBP_Interact OtherActor))
  (Variables|Default|SetInteract%20Actor _asbp_interact)
  (Class|BPIInteract|BeginOverlap(Message) _asbp_interact))

(event OnComponentEndOverlap(CapsuleInteract)
  (params (OverlappedComponent :type Primitive%20Component%20Object%20Reference) (OtherActor :type Actor%20Object%20Reference) (OtherComp :type Primitive%20Component%20Object%20Reference) (OtherBodyIndex :type Integer))
  ;[1 1 1] Interact
  (bind _asbp_interact (Utilities|Casting|CastToBP_Interact OtherActor))
  (Variables|Default|SetInteract%20Actor 0)
  (Class|BPIInteract|EndOverlap(Message) _asbp_interact))

(event Input|EnhancedActionEvents|EnhancedInputActionIA_Walk
  (params (ActionValue :type Vector%202D%20Structure) (ElapsedSeconds :type Float%20%28double-precision%29) (TriggeredSeconds :type Float%20%28double-precision%29) (InputAction :type Input%20Action%20Object%20Reference :default "/Game/05-Inputs/InputActions/IA_Walk.IA_Walk"))
  (Pawn|Input|AddMovementInput (Transformation|GetActorRightVector) (.x ActionValue) false)
  (Pawn|Input|AddMovementInput (Transformation|GetActorForwardVector) (.y ActionValue) false))

(event Input|EnhancedActionEvents|EnhancedInputActionIA_Look
  (params (ActionValue :type Vector%202D%20Structure) (ElapsedSeconds :type Float%20%28double-precision%29) (TriggeredSeconds :type Float%20%28double-precision%29) (InputAction :type Input%20Action%20Object%20Reference :default "/Game/05-Inputs/InputActions/IA_Look.IA_Look"))
  (if (not (Variables|Default|Getb_IsOnMenuSetting))
    (bind _result (Math|Float|NegateFloat (.x ActionValue))
      (:%20%20
        (Pawn|Input|AddControllerYawInput _result)
        (Pawn|Input|AddControllerPitchInput (.y ActionValue))))))

(event Input|EnhancedActionEvents|EnhancedInputActionIA_PaintMenu
  (params (ActionValue :type Boolean) (ElapsedSeconds :type Float%20%28double-precision%29) (TriggeredSeconds :type Float%20%28double-precision%29) (InputAction :type Input%20Action%20Object%20Reference :default "/Game/05-Inputs/InputActions/IA_PaintMenu.IA_PaintMenu"))
  (bind _maskref (Variables|Default|GetMaskRef))
  (bind _scene (Variables|Default|GetScene))
  (bind _wg_paintref (Variables|Default|GetWG_PaintRef))
  (bind _arrow (Variables|/Game/01-Bluprints/Player/Plane_Blueprint.Plane_Blueprint_C|GetArrow _maskref))
  (:Started
    (if (Variables|Default|Getb_IsOnMenuSetting)
      (Widget|RemovefromParent _wg_paintref)
      (Transformation|SetRelativeLocation (Variables|Default|GetCube) "0, 0, 0" false false)
      (Variables|Default|Setb_IsOnMenuSetting false)
      (Variables|/Script/Engine.PlayerController|SetbShowMouseCursor (Game|GetPlayerController 0) false)
      (Transformation|SetWorldLocationAndRotation (Variables|Default|GetCamera) (Transformation|GetWorldLocation _scene) (Transformation|GetWorldRotation _scene) false false)
      (Default|CalculatePercentColor (Variables|Default|GetRVTReft))
      (else
        (UserInterface|Viewport|AddtoViewport _wg_paintref 0)
        (Variables|Default|Setb_IsOnMenuSetting true)
        (Variables|/Script/Engine.PlayerController|SetbShowMouseCursor (Game|GetPlayerController 0) true)
        (Transformation|SetWorldLocationAndRotation (Variables|Default|GetCamera) (Transformation|GetWorldLocation _arrow) (Transformation|GetWorldRotation _arrow) false false)))))

(event Input|EnhancedActionEvents|EnhancedInputActionIA_Click
  (params (ActionValue :type Boolean) (ElapsedSeconds :type Float%20%28double-precision%29) (TriggeredSeconds :type Float%20%28double-precision%29) (InputAction :type Input%20Action%20Object%20Reference :default "/Game/05-Inputs/InputActions/IA_Click.IA_Click"))
  (bind _returnvalue (Game|GetPlayerController 0))
  (bind (_worldlocation _worlddirection) (Game|Player|ConvertMouseLocationToWorldSpace _returnvalue))
  (:Started
    (bind _outhit (Collision|LineTraceByChannel _worldlocation (+ _worldlocation (* _worlddirection 5e+02)) "TraceTypeQuery1" false 0 "None"))
    (Transformation|SetWorldLocation (Variables|Default|GetCube) (.Location (Collision|BreakHitResult _outhit)) false false)
    (Variables|Default|SetActualPos (Transformation|GetWorldLocation (Variables|Default|GetCube)))
    (Variables|Default|Setb_IsClicking true))
  (:Canceled
    (Variables|Default|Setb_IsClicking false :!label _label))
  (:Completed
    (goto _label)))

(event Input|EnhancedActionEvents|EnhancedInputActionIA_Interact
  (params (ActionValue :type Boolean) (ElapsedSeconds :type Float%20%28double-precision%29) (TriggeredSeconds :type Float%20%28double-precision%29) (InputAction :type Input%20Action%20Object%20Reference :default "/Game/05-Inputs/InputActions/IA_Interact.IA_Interact"))
  ;[1 1 1] Interact
  (:Started
    (bind _interact_actor (Variables|Default|GetInteract%20Actor)
      (:then
        (Class|BPIInteract|Interact(Message) _interact_actor))
      (:else))))

(event EventBeginPlay
  (Game|Player|SetViewTargetwithBlend (Game|GetPlayerController 0) self 0.0 "VTBlend_Linear" 0.0 false)
  (Variables|Default|SetInitPos (Variables|/Script/Engine.SceneComponent|GetRelativeLocation (Variables|Default|GetCube)))
  (bind _returnvalue (Actor|GetActorOfClass "/Game/01-Bluprints/Player/Plane_Blueprint.Plane_Blueprint_C"))
  (Variables|Default|SetMaskRef _returnvalue)
  (bind _returnvalue_2 (Actor|GetActorOfClass "/Game/01-Bluprints/Player/Materials/BP_RVT_Volume.BP_RVT_Volume_C"))
  (bind _output_get (Variables|Default|SetRVTReft _returnvalue_2))
  (Variables|/Game/01-Bluprints/Player/Materials/BP_RVT_Volume.BP_RVT_Volume_C|SetPlayer _output_get self)
  (bind _returnvalue_3 (UserInterface|CreateWidget "/Game/09-Widgets/WG_Paint.WG_Paint_C" 0 self))
  (Variables|Default|SetWG_PaintRef _returnvalue_3))

(event EventTick
  (params (DeltaSeconds :type Float%20%28single-precision%29))
  (bind _returnvalue (Game|GetPlayerController 0))
  (bind (_worldlocation _worlddirection) (Game|Player|ConvertMouseLocationToWorldSpace _returnvalue))
  (if (and (Variables|Default|Getb_IsClicking) (Variables|Default|Getb_IsOnMenuSetting))
    (bind _outhit (Collision|LineTraceByChannel _worldlocation (+ _worldlocation (* _worlddirection 9999999.0)) "TraceTypeQuery1" false 0 "None"))
    (Transformation|SetWorldLocation (Variables|Default|GetCube) (select true (Math|Interpolation|VInterpTo (Variables|Default|GetActualPos) (.Location (Collision|BreakHitResult _outhit)) DeltaSeconds 1e+01) (.Location (Collision|BreakHitResult _outhit))) false false)
    (Variables|Default|SetActualPos (Transformation|GetWorldLocation (Variables|Default|GetCube)))))

(fn ConstructionScript)
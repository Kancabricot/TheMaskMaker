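; BP_RVT_Volume paints color into render targets and scores how much of the area is blue, red or green.
; Each tick it draws a dynamic material, whose channel parameters ChangeColor sets, into catcher and score render targets, which are cleared on start or Clear.
; CalculatePercentColor reads back score pixels, counts each by dominant channel priority, and writes percentages to the Player, printing them.
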(event Custom|Clear
  (Rendering|ClearRenderTarget2D "/Game/01-Bluprints/Player/Materials/RT_Catcher.RT_Catcher" "(R=1.000000,G=1.000000,B=1.000000,A=1.000000)")
  (Rendering|ClearRenderTarget2D "/Game/01-Bluprints/Player/Materials/RT_ScoreCatcher.RT_ScoreCatcher")
  (CallFunction|CalculatePercentColor))

(event Custom|ChangeColor
  (params (Red :type Boolean) (Blue :type Boolean) (Green :type Boolean))
  (bind _materialinstance (Variables|Default|GetMaterialInstance))
  (Rendering|Material|SetScalarParameterValue _materialinstance "GreenChannel" (select Green 1.0 0.0) :!class /Script/Engine.MaterialInstanceDynamic)
  (Rendering|Material|SetScalarParameterValue _materialinstance "BlueChannel" (select Blue 1.0 0.0) :!class /Script/Engine.MaterialInstanceDynamic)
  (Rendering|Material|SetScalarParameterValue _materialinstance "RedChannel" (select Red 1.0 0.0) :!class /Script/Engine.MaterialInstanceDynamic))

(event Custom|CalculatePercentColor
  (bind _player (Variables|Default|GetPlayer))
  (Variables|Default|SetNBPixel 0)
  (Variables|Default|SetNBBlue 0)
  (Variables|Default|SetNBRed 0)
  (Variables|Default|SetNBGreen 0)
  (bind _outsamples (Class|KismetRenderingLibrary|ReadRenderTarget "/Game/01-Bluprints/Player/Materials/RT_ScoreCatcher.RT_ScoreCatcher" true))
  (Variables|Default|SetRT_Pixel _outsamples)
  (Variables|Default|SetNBPixel (- (Utilities|Array|Length _outsamples) 600))
  (for _array_element (Variables|Default|GetRT_Pixel)
    (if (> (.B (Math|Color|BreakColor _array_element)) 0)
      (Variables|Default|SetNBBlue (+ (Variables|Default|GetNBBlue) 1))
      (elif (> (.G (Math|Color|BreakColor _array_element)) 0)
        (Variables|Default|SetNBGreen (+ (Variables|Default|GetNBGreen) 1))
        (elif (> (.R (Math|Color|BreakColor _array_element)) 0)
          (Variables|Default|SetNBRed (+ (Variables|Default|GetNBRed) 1))))))
  (bind _output_get (Variables|/Game/01-Bluprints/Player/BP_Player.BP_Player_C|SetPercentBlue _player (/ (* (Variables|Default|GetNBBlue) 100) (Variables|Default|GetNBPixel))))
  (bind _output_get_2 (Variables|/Game/01-Bluprints/Player/BP_Player.BP_Player_C|SetPercentGreen _player (/ (* (Variables|Default|GetNBGreen) 100) (Variables|Default|GetNBPixel))))
  (bind _output_get_3 (Variables|/Game/01-Bluprints/Player/BP_Player.BP_Player_C|SetPercentRed _player (/ (* (Variables|Default|GetNBRed) 100) (Variables|Default|GetNBPixel))))
  (Development|PrintString (Utilities|String|Append (Utilities|String|ToString(Integer) _output_get) " % Blue" " 
" (Utilities|String|ToString(Integer) _output_get_3) " % Red" " 
" (Utilities|String|ToString(Integer) _output_get_2) " % Green") true true "(R=1.000000,G=0.000000,B=0.628946,A=1.000000)" 1e+01))

(event EventBeginPlay
  (bind _returnvalue (Rendering|Material|CreateDynamicMaterialInstance (Variables|Default|GetMaterial) "None" "None" :!class /Script/Engine.KismetMaterialLibrary))
  (Variables|Default|SetMaterialInstance _returnvalue)
  (Rendering|ClearRenderTarget2D "/Game/01-Bluprints/Player/Materials/RT_Catcher.RT_Catcher" "(R=1.000000,G=1.000000,B=1.000000,A=1.000000)")
  (Rendering|ClearRenderTarget2D "/Game/01-Bluprints/Player/Materials/RT_ScoreCatcher.RT_ScoreCatcher")
  (CallFunction|CalculatePercentColor))

(event EventTick
  (params (DeltaSeconds :type Float%20%28single-precision%29))
  (bind _materialinstance (Variables|Default|GetMaterialInstance))
  (Rendering|DrawMaterialtoRenderTarget "/Game/01-Bluprints/Player/Materials/RT_Catcher.RT_Catcher" _materialinstance)
  (Rendering|DrawMaterialtoRenderTarget "/Game/01-Bluprints/Player/Materials/RT_ScoreCatcher.RT_ScoreCatcher" _materialinstance))

(fn ConstructionScript)
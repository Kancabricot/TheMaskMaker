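; BP_Sentry is a sentry that checks the colors of the player's mask and changes post when it approves.
; Sphere overlap compares the player's red, green and blue percentages against the sentry's min/max ranges.
; A valid mask plays an agreeing montage, then, unless already moving, has AIC_Sentry send it between guard and door positions.
; An invalid mask only plays a head-shake montage, with debug prints throughout.
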(event OnComponentBeginOverlap(Sphere)
  (params (OverlappedComponent :type Primitive%20Component%20Object%20Reference) (OtherActor :type Actor%20Object%20Reference) (OtherComp :type Primitive%20Component%20Object%20Reference) (OtherBodyIndex :type Integer) (bFromSweep :type Boolean) (SweepResult :type Hit%20Result%20Structure%20%28by%20ref%29))
  (bind _asbp_player (Utilities|Casting|CastToBP_Player OtherActor))
  (bind _is_mask_valid (CallFunction|CheckifMaskIsValid (Variables|/Game/01-Bluprints/Player/BP_Player.BP_Player_C|GetPercentBlue _asbp_player) (Variables|/Game/01-Bluprints/Player/BP_Player.BP_Player_C|GetPercentGreen _asbp_player) (Variables|/Game/01-Bluprints/Player/BP_Player.BP_Player_C|GetPercentRed _asbp_player)))
  (if _is_mask_valid
    (CallFunction|ValidMask)
    (else
      (CallFunction|UnvalidMask))))

(event OnComponentEndOverlap(Sphere)
  (params (OverlappedComponent :type Primitive%20Component%20Object%20Reference) (OtherActor :type Actor%20Object%20Reference) (OtherComp :type Primitive%20Component%20Object%20Reference) (OtherBodyIndex :type Integer)))

(event Custom|Valid%20Mask
  (Development|PrintString "Hello")
  (Animation|Montage|PlayMontage (Variables|Character|GetMesh) "/Game/03-Meshs/Animations/Agreeing_mixamo_com_Montage.Agreeing_mixamo_com_Montage"
    (:OnCompleted
      (if (not (Variables|Default|Getb_isMoving))
        (Default|NextLocation (Variables|Default|GetAIC%20Sentry) (select (Variables|Default|Getb_isAtDoorPos) (Transformation|GetWorldLocation (Variables|Default|GetGuard%20Pos)) (Transformation|GetWorldLocation (Variables|Default|GetDoor%20Pos))))))))

(event Custom|Unvalid%20Mask
  (Development|PrintString "Hello" true true "(R=1.000000,G=0.000000,B=0.040488,A=1.000000)")
  (Animation|Montage|PlayMontage (Variables|Character|GetMesh) "/Game/03-Meshs/Animations/Thoughtful_Head_Shake_mixamo_com_Montage.Thoughtful_Head_Shake_mixamo_com_Montage"
    (:OnCompleted
      (Development|PrintString "Hello" true true "(R=1.000000,G=0.421689,B=0.000000,A=1.000000)"))))

(event EventBeginPlay
  (bind _asaic_sentry (Utilities|Casting|CastToAIC_Sentry (AI|GetAIController self)))
  (Variables|/Game/01-Bluprints/Sentry/AIC_Sentry.AIC_Sentry_C|SetSentry _asaic_sentry self)
  (Variables|Default|SetAIC%20Sentry _asaic_sentry))

(fn ConstructionScript)

(fn CheckifMaskIsValid
  (params (Blue :type Integer) (Green :type Integer) (Red :type Integer))
  (if (and (>= Blue (Variables|Default|GetBlueMin)) (<= Blue (Variables|Default|GetBlueMax)))
    (if (and (>= Green (Variables|Default|GetGreenMin)) (<= Green (Variables|Default|GetGreenMax)))
      (if (and (>= Red (Variables|Default|GetRedMin)) (<= Red (Variables|Default|GetRedMax)))
        (Development|PrintString "Hello" true true "(R=0.000000,G=0.490771,B=1.000000,A=1.000000)")
        (return true)
        (else
          (Development|PrintString "Hello" true true "(R=0.000000,G=1.000000,B=0.492241,A=1.000000)")
          (return false))))))
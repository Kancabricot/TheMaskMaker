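; Double door actor that swings its two leaves open when BP_Player enters its trigger box.
; BIsOpen sets the starting pose, gates opening on begin overlap when false and reversing on end overlap when true; this graph never changes it.
; A timeline lerps the leaves to mirrored quarter-turn yaws and, on finishing, destroys the referenced spawner if valid.
; The CanBeOppen-gated play and reverse branches are disconnected.
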(event OnComponentBeginOverlap(Box)
  (params (OverlappedComponent :type Primitive%20Component%20Object%20Reference) (OtherActor :type Actor%20Object%20Reference) (OtherComp :type Primitive%20Component%20Object%20Reference) (OtherBodyIndex :type Integer) (bFromSweep :type Boolean) (SweepResult :type Hit%20Result%20Structure%20%28by%20ref%29))
  (Utilities|Casting|CastToBP_Player OtherActor)
  (if (not (Variables|Default|Getb_isOpen))
    (bind _newtrack_0 (Timeline|Timeline PlayFromStart)
      (:Update
        (Transformation|SetRelativeRotation (Variables|Default|GetSM_LeftDoor) (Math|Rotator|Lerp(Rotator) "0, 0, 0" "0.000000,-90.000000,0.000000" _newtrack_0 true) false false)
        (Transformation|SetRelativeRotation (Variables|Default|GetSM_RightDoor) (Math|Rotator|Lerp(Rotator) "0, 0, 0" "0.000000,90.000000,0.000000" _newtrack_0 true) false false))
      (:Finished
        (bind _spawner_ref (Variables|Default|GetSpawner%20Ref)
          (:then
            (Actor|DestroyActor _spawner_ref))
          (:else))))))

(event OnComponentEndOverlap(Box)
  (params (OverlappedComponent :type Primitive%20Component%20Object%20Reference) (OtherActor :type Actor%20Object%20Reference) (OtherComp :type Primitive%20Component%20Object%20Reference) (OtherBodyIndex :type Integer))
  (Utilities|Casting|CastToBP_Player OtherActor)
  (if (Variables|Default|Getb_isOpen)
    (bind _newtrack_0 (Timeline|Timeline Reverse)
      (:Update
        (Transformation|SetRelativeRotation (Variables|Default|GetSM_LeftDoor) (Math|Rotator|Lerp(Rotator) "0, 0, 0" "0.000000,-90.000000,0.000000" _newtrack_0 true) false false)
        (Transformation|SetRelativeRotation (Variables|Default|GetSM_RightDoor) (Math|Rotator|Lerp(Rotator) "0, 0, 0" "0.000000,90.000000,0.000000" _newtrack_0 true) false false))
      (:Finished
        (bind _spawner_ref (Variables|Default|GetSpawner%20Ref)
          (:then
            (Actor|DestroyActor _spawner_ref))
          (:else))))))

(event EventBeginPlay
  (bind _b_isopen (Variables|Default|Getb_isOpen))
  (Transformation|SetRelativeRotation (Variables|Default|GetSM_LeftDoor) (select _b_isopen "0.000000,-90.000000,0.000000" "0, 0, 0") false false)
  (Transformation|SetRelativeRotation (Variables|Default|GetSM_RightDoor) (select _b_isopen "0.000000,90.000000,0.000000" "0, 0, 0") false false))

(fn ConstructionScript)
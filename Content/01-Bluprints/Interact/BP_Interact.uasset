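; BP_Interact is a collectible actor that grants paint color to the player on interaction.
; Interact passes its R, G and B values to the player's GetColorPaint, spawns the pickup Niagara effect at the cube, then destroys the actor.
; BeginOverlap and EndOverlap events toggle an outline overlay material on the cube.
; From BeginPlay, a timeline animates an idle vertical bob from the starting location.
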(event Custom|StartAnimationIdle
  (Components|Timeline|SetPlayRate (Variables|Default|GetTL_Idle) (/ 0.5 1.0))
  (Variables|Default|SetStartLocation (Transformation|GetActorLocation))
  (bind _newtrack_0 (Timeline|TL_Idle PlayFromStart)
    (:Update
      (Transformation|SetActorLocation (Math|Vector|Lerp(Vector) (Variables|Default|GetStartLocation) (+ (Variables|Default|GetStartLocation) "0.000000,0.000000,25.000000") _newtrack_0) false false))))

(event EventBeginPlay
  (CallFunction|StartAnimationIdle))

(event Collision|EventActorBeginOverlap
  (params (OtherActor :type Actor%20Object%20Reference)))

(event EventTick
  (params (DeltaSeconds :type Float%20%28single-precision%29)))

(event EventInteract
  (params (PlayerRef :type BP%20Player%20Object%20Reference))
  (bind _output_get (Variables|Default|SetPlayer%20Ref PlayerRef))
  (Default|GetColorPaint _output_get (Variables|Default|GetR) (Variables|Default|GetB) (Variables|Default|GetG))
  (Niagara|SpawnSystematLocation "/Game/04-VFX/04-NiagaraSystem/NS_Collectible_Pickup.NS_Collectible_Pickup" (Transformation|GetWorldLocation (Variables|Default|GetCube)))
  (Actor|DestroyActor))

(event EventBeginOverlap
  (Rendering|Material|SetOverlayMaterial (Variables|Default|GetCube) "/Game/06-Materials/Outlines/M_Outline.M_Outline" :!class /Script/Engine.MeshComponent))

(event EventEndOverlap
  (Rendering|Material|SetOverlayMaterial (Variables|Default|GetCube) 0 :!class /Script/Engine.MeshComponent))

(fn ConstructionScript)